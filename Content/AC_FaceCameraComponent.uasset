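; Actor component that billboards its owning actor toward player 0's pawn.
; Every Tick it builds a rotation with local Y fixed straight down and local Z aimed horizontally at the pawn, then applies it to the owner.
; The rotation passes through RInterpTo with no interp speed set, so it snaps rather than eases.
; An unused MakeRotFromZ alternative remains in the graph.
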(event EventTick
  (params (DeltaSeconds :type Float%20%28single-precision%29))
  (bind _returnvalue (Components|GetOwner))
  (Transformation|SetActorRotation _returnvalue (Math|Interpolation|RInterpTo (Transformation|GetActorRotation _returnvalue) (Class|KismetMathLibrary|MakeRotfromYZ (Math|Vector|VectorDown) (- (Transformation|GetActorLocation (Game|Player|GetPlayerPawn 0)) (Transformation|GetActorLocation _returnvalue))) DeltaSeconds 0.0)))